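; BP_Block_Wall is a breakable wall block built on a Destructible component that reacts to hits from BP_Ball.
; On fracture, it enables gravity and changes collision to ignore physics bodies while blocking destructibles and static world geometry.
; A ball hit destroys the whole actor after a short delay.
; A leftover debug print on the hit path is disconnected.
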(event OnComponentHit(Destructible)
  (params (HitComponent :type Primitive%20Component%20Object%20Reference) (OtherActor :type Actor%20Object%20Reference) (OtherComp :type Primitive%20Component%20Object%20Reference) (NormalImpulse :type Vector :default "0, 0, 0") (Hit :type Hit%20Result%20Structure%20%28by%20ref%29))
  (Utilities|Casting|CastToBP_Ball OtherActor)
  (Utilities|FlowControl|Delay 1.5)
  (Actor|DestroyActor))

(event OnComponentFracture(Destructible)
  (params (HitPoint :type Vector%20%28by%20ref%29 :default "0, 0, 0") (HitDirection :type Vector%20%28by%20ref%29 :default "0, 0, 0"))
  (Physics|SetEnableGravity (Variables|Default|GetDestructible) true)
  (Collision|SetCollisionResponsetoChannel (Variables|Default|GetDestructible) "ECC_PhysicsBody" "ECR_Ignore")
  (Collision|SetCollisionResponsetoChannel (Variables|Default|GetDestructible) "ECC_Destructible" "ECR_Block")
  (Collision|SetCollisionResponsetoChannel (Variables|Default|GetDestructible) "ECC_WorldStatic" "ECR_Block"))

(fn ConstructionScript)