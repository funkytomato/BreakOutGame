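; BOGameMode is a Game Mode Blueprint that tracks lives, score and game-over state.
; On BeginPlay it creates the HUD widget and resets the game, then pushes lives and points changes straight to that widget.
; UpdateScore clamps the total at zero, and LifeLost applies a score penalty before decrementing lives.
; A life lost with none remaining triggers GameOver, which quits the game after a short delay.
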(event Custom|Reset
  (bind _maxlives (Variables|Default|GetMaxLives))
  (bind _hud (Variables|Default|GetHUD))
  ;[1 1 1] Reset Game
  (Variables|Default|SetLives _maxlives)
  (Variables|/Game/MyContent/Blueprints/HUD.HUD_C|SetLives _hud _maxlives)
  (Variables|/Game/MyContent/Blueprints/HUD.HUD_C|SetPoints _hud 0)
  (Variables|Default|SetCurrentPoints 0)
  (Variables|Default|SetGameOver? false))

(event Custom|UpdateScore
  (params (Points :type Integer))
  ;[1 1 1] Update Score
  (if (<= (+ Points (Variables|Default|GetCurrentPoints)) 0)
    (Variables|Default|SetCurrentPoints 0)
    (else
      (Variables|Default|SetCurrentPoints (+ Points (Variables|Default|GetCurrentPoints)))))
  (Variables|/Game/MyContent/Blueprints/HUD.HUD_C|SetPoints (Variables|Default|GetHUD) (Variables|Default|GetCurrentPoints)))

(event Custom|LifeLost
  ;[1 1 1] Life Lost
  (CallFunction|UpdateScore -500)
  (if (<= (Variables|Default|GetLives) 0)
    (CallFunction|GameOver)
    (else
      (bind _output_get (Variables|Default|SetLives (- (Variables|Default|GetLives) 1)))
      (Variables|/Game/MyContent/Blueprints/HUD.HUD_C|SetLives (Variables|Default|GetHUD) _output_get))))

(event Custom|GameOver
  ;[1 1 1] Game Over
  (Variables|Default|SetGameOver? true)
  (Utilities|FlowControl|Delay 5.0)
  (Game|QuitGame 0 "Quit" false))

(event EventBeginPlay
  ;[1 1 1] Add HUD
  (bind _returnvalue (UserInterface|CreateWidget "/Game/MyContent/Blueprints/HUD.HUD_C"))
  (bind _output_get (Variables|Default|SetHUD _returnvalue))
  (UserInterface|Viewport|AddtoViewport _output_get 0)
  (CallFunction|Reset))

(fn ConstructionScript)