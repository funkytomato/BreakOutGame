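; BP_PlayerPaddle is the player-controlled paddle that spawns and launches the ball.
; Horizontal axis input moves it by applying an X impulse scaled by Speed to the physics Paddle component.
; NewBall spawns a BP_Ball at the Arrow component's transform on BeginPlay, unless the cached BOGameMode reports game over.
; The Fire action launches the current ball if it is valid and not yet active.
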(event Custom|New%20Ball
  ;[1 1 1] Spawn Ball
  (if (not (Variables|/Game/MyContent/Blueprints/BOGameMode.BOGameMode_C|GetGameOver? (Variables|Default|GetGameMode)))
    (bind _returnvalue (Game|SpawnActorfromClass "/Game/MyContent/Blueprints/BP_Ball.BP_Ball_C" (Transformation|GetWorldTransform (Variables|Default|GetArrow)) "Undefined" 0 0))
    (Variables|Default|SetBall _returnvalue)))

(event EventBeginPlay
  ;[1 1 1] Create a Ball at Start
  ;;[1 1 1] Get Game Mode
  (bind _asbogame_mode (Utilities|Casting|CastToBOGameMode (Game|GetGameMode)))
  (Variables|Default|SetGameMode _asbogame_mode)
  (CallFunction|NewBall))

(event Input|ActionEvents|InputActionFire
  (params (Key :type Key%20Structure :default "None"))
  (bind _ball (Variables|Default|GetBall))
  ;[1 1 1] Launch FireBall
  (:Pressed
    (if (and (Utilities|IsValid _ball) (not (Variables|/Game/MyContent/Blueprints/BP_Ball.BP_Ball_C|GetActive _ball)))
      (Default|LaunchBall (Variables|Default|GetBall)))))

(event Input|AxisEvents|InputAxisHorizontalMovement
  (params (AxisValue :type Float%20%28single-precision%29))
  ;[1 1 1] Paddle Movement
  (Physics|AddImpulse (Variables|Default|GetPaddle) (Math|Vector|MakeVector (* AxisValue (Variables|Default|GetSpeed)) 0.0 0.0) "None" false))

(fn ConstructionScript)