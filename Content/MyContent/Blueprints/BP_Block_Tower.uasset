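; BP_Block_Tower is a destructible block tower actor that crumbles with a sound when fractured, then removes itself.
; On component fracture it enables gravity and changes collision to ignore physics bodies while blocking destructibles and static world.
; It then calls a radial impulse from just above the destructible's location, plays a 2D crumble sound and destroys the actor after a short delay.
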(event OnComponentFracture(Destructible)
  (params (HitPoint :type Vector%20%28by%20ref%29 :default "0, 0, 0") (HitDirection :type Vector%20%28by%20ref%29 :default "0, 0, 0"))
  (bind _destructible (Variables|Default|GetDestructible))
  (bind _returnvalue (Transformation|GetWorldLocation _destructible))
  ;[1 1 1] Set Fracture objects Collision Responder and Make a Sound on destruction
  (Physics|SetEnableGravity (Variables|Default|GetDestructible) true)
  (Collision|SetCollisionResponsetoChannel (Variables|Default|GetDestructible) "ECC_PhysicsBody" "ECR_Ignore")
  (Collision|SetCollisionResponsetoChannel (Variables|Default|GetDestructible) "ECC_Destructible" "ECR_Block")
  (Collision|SetCollisionResponsetoChannel (Variables|Default|GetDestructible) "ECC_WorldStatic" "ECR_Block")
  (Physics|AddRadialImpulse _destructible (Math|Vector|MakeVector (.x _returnvalue) (.y _returnvalue) (+ (.z _returnvalue) 5e+01)) 0.0 0.0 "RIF_Linear" false)
  (Audio|PlaySound2D "/Game/MyContent/Audio/Crumble.Crumble" 1.0 1.0 0.0 0 0)
  (Utilities|FlowControl|Delay 3.0)
  (Actor|DestroyActor))

(fn ConstructionScript)